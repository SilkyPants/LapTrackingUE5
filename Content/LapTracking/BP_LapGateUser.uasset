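; BP_LapGateUser tracks an entity's progress through numbered lap gates and counts completed laps.
; EnterGate accepts only the gate matching NextGate, notifies it through OnPassed, then advances the index modulo MaxGates, enforcing gate order.
; When the index wraps to zero, it increments NumLaps and calls OnLapPassed on that final gate, returning the result.
; BeginPlay starts the sequence at gate zero, and Tick is unused.
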(event EventBeginPlay
  (Variables|Default|SetNextGate 0))

(event EventTick
  (params (DeltaSeconds :type Float%20%28single-precision%29)))

(fn EnterGate
  (params (Gate :type BP%20Lap%20Gate%20Object%20Reference))
  ;[1 1 1] Check this is the next gate
  (if (== (Variables|/Game/LapTracking/BP_LapGate.BP_LapGate_C|GetGateNumber Gate) (Variables|Default|GetNextGate))
    ;[1 1 1] Increment and wrap gate counter
    (Default|OnPassed Gate)
    (bind _result (Math|Integer|IncrementInt (Variables|Default|GetNextGate))
      (:%20%20
        (bind _output_get (Variables|Default|SetNextGate (Math|Integer|%(Integer) _result (Variables|Default|GetMaxGates))))
        ;[1 1 1] Check for a complete lap
        (if (== _output_get 0)
          (Math|Integer|IncrementInt (Variables|Default|GetNumLaps)
            (:%20%20
              (bind _emitters (Default|OnLapPassed Gate))
              (return _emitters))))))))